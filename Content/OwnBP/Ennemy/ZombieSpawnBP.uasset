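; ZombieSpawnBP is an enemy spawner that spawns actors at its own transform when the game mode signals a respawn.
; On BeginPlay it binds SpawnEnemy to the TrenchesGameMod respawn notification.
; SpawnEnemy spawns batches of 20, repeating after a delay until the EnemySpawn counter reaches 100, and prints each count.
; The counter is never reset here, so later notifications after completion spawn only one batch.
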(event Custom|SpawnEnemy
  ;[1 1 1] When receiving the notification of "respawn enemy" => spawn 100 enemies, 20 / 20.
  (Utilities|FlowControl|Sequence :!label _label
    (:then_0
      (for _index (range 1 20)
        (Game|SpawnActorfromClass "/Game/OwnBP/Ennemy/ZombieIA.ZombieIA_C" (Transformation|GetActorTransform) "AdjustIfPossibleButAlwaysSpawn" "MultiplyWithRoot" 0 0)
        (bind _result (Math|Integer|IncrementInt (Variables|Default|GetEnemySpawn))
          (:%20%20
            (Variables|Default|SetEnemySpawn _result)
            (Development|PrintString (Utilities|String|ToString(Integer) (Variables|Default|GetEnemySpawn)))))))
    (:then_1
      (Utilities|FlowControl|Delay 1e+01)
      (if (< (Variables|Default|GetEnemySpawn) 100)
        (goto _label)))))

(event EventBeginPlay
  (bind _astrenches_game_mod (Utilities|Casting|CastToTrenchesGameMod (Game|GetGameMode)))
  ;[1 1 1] When receiving the notification of "respawn enemy" => spawn 100 enemies, 20 / 20.
  (EventDispatchers|BindEventtoRespawnEnemy _astrenches_game_mod (delegate Custom|SpawnEnemy)))

(fn ConstructionScript)