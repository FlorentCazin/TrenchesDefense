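; Animation notify that lands an AI character's attack at a chosen frame of its animation in Trenches Defense.
; When fired, it finds the TrenchesDefenseCharacter that owns the mesh and that character's TrenchesDefenseAIController.
; It reads TargetActor from the controller's blackboard and, if that is a valid TrenchesDefenseCharacter, passes it to the controller's Attack function.
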(fn ReceivedNotify
  (params (MeshComp :type Skeletal%20Mesh%20Component%20Object%20Reference) (Animation :type Anim%20Sequence%20Base%20Object%20Reference) (EventReference :type Anim%20Notify%20Event%20Reference%20Structure%20%28by%20ref%29))
  (bind _astrenches_defense_character (Utilities|Casting|CastToTrenchesDefenseCharacter (Components|GetOwner MeshComp)))
  (bind _astrenches_defense_aicontroller (Utilities|Casting|CastToTrenchesDefenseAIController (Pawn|GetController _astrenches_defense_character)))
  (if (Utilities|IsValid (AI|Components|Blackboard|GetValueasObject (AI|GetBlackboard _astrenches_defense_aicontroller) (Variables|Default|GetTargetActor)))
    (bind _astrenches_defense_character_2 (Utilities|Casting|CastToTrenchesDefenseCharacter (AI|Components|Blackboard|GetValueasObject (AI|GetBlackboard _astrenches_defense_aicontroller) (Variables|Default|GetTargetActor))))
    (Class|TrenchesDefenseAIController|Attack _astrenches_defense_aicontroller _astrenches_defense_character_2)
    (return (Utilities|IsValid (AI|Components|Blackboard|GetValueasObject (AI|GetBlackboard _astrenches_defense_aicontroller) (Variables|Default|GetTargetActor))))))