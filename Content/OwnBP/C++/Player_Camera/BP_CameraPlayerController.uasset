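; Player controller for the camera pawn, routing Enhanced Input to soldier placement and editing, camera zoom, rotation and the in-game menu.
; BeginPlay saves the default soldier spawn location, adds the input mapping context and creates the preview, speaking and basic information widgets.
; Spawn/edit clicks call OnLeftClick, then start or stop the soldier preview depending on selection validity, while cancel undoes the last action.
; Rotation input only sets a right-click flag, and a FlipFlop toggles the menu.
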(event Input|EnhancedActionEvents|EnhancedInputActionIA_SpawningEditSystem
  (params (ActionValue :type Boolean) (ElapsedSeconds :type Float%20%28double-precision%29) (TriggeredSeconds :type Float%20%28double-precision%29) (InputAction :type Input%20Action%20Object%20Reference :default "/Game/OwnBP/C++/Player_Camera/Inputs/IA_SpawningEditSystem.IA_SpawningEditSystem"))
  ;[1 1 1] spawning/edit system called + preview
  (Class|CameraPlayerController|OnLeftClick)
  (bind _returnvalue (Actor|GetActorOfClass "/Game/OwnBP/C++/Allies/Preview/BP_TrenchesDefensePreviewCharacter.BP_TrenchesDefensePreviewCharacter_C"))
  (if (and (== (Utilities|IsValid (Variables|/Script/TrenchesDefense.TrenchesDefensePreviewCharacter|GetCharacterToPreview _returnvalue)) false) (Utilities|IsValid (Variables|Default|GetSoldierToSpawn)))
    (Default|CallOnClickSoldierPreview (Variables|Default|GetSoldierToSpawn))
    (elif (and (== (Utilities|IsValid (Variables|Default|GetSoldierToSpawn)) false) (Utilities|IsValid (Variables|/Script/TrenchesDefense.TrenchesDefensePreviewCharacter|GetCharacterToPreview _returnvalue)))
      (Default|CallOnStopSelecting))))

(event Input|EnhancedActionEvents|EnhancedInputActionIA_OpenMenu
  (params (ActionValue :type Boolean) (ElapsedSeconds :type Float%20%28double-precision%29) (TriggeredSeconds :type Float%20%28double-precision%29) (InputAction :type Input%20Action%20Object%20Reference :default "/Game/OwnBP/C++/Player_Camera/Inputs/IA_OpenMenu.IA_OpenMenu"))
  ;[1 1 1] OpenMenu
  (Utilities|FlowControl|FlipFlop
    (:A
      (bind _returnvalue (UserInterface|CreateWidget "/Game/OwnBP/C++/menu/BP_MenuInGameWidget.BP_MenuInGameWidget_C"))
      (UserInterface|Viewport|AddtoViewport _returnvalue 0)
      (Widget|SetVisibility _returnvalue "Visible"))
    (:B
      (Widget|RemovefromParent _returnvalue))))

(event Input|EnhancedActionEvents|EnhancedInputActionIA_RotateCameraStart
  (params (ActionValue :type Boolean) (ElapsedSeconds :type Float%20%28double-precision%29) (TriggeredSeconds :type Float%20%28double-precision%29) (InputAction :type Input%20Action%20Object%20Reference :default "/Game/OwnBP/C++/Player_Camera/Inputs/IA_RotateCameraStart.IA_RotateCameraStart"))
  ;[1 1 1] rotation giving the priority for the first axe trigged
  (Variables|Default|SetRightClickPressed true))

(event Input|EnhancedActionEvents|EnhancedInputActionIA_RotateCameraStop
  (params (ActionValue :type Boolean) (ElapsedSeconds :type Float%20%28double-precision%29) (TriggeredSeconds :type Float%20%28double-precision%29) (InputAction :type Input%20Action%20Object%20Reference :default "/Game/OwnBP/C++/Player_Camera/Inputs/IA_RotateCameraStop.IA_RotateCameraStop"))
  ;[1 1 1] rotation giving the priority for the first axe trigged
  (Variables|Default|SetRightClickPressed false))

(event Input|EnhancedActionEvents|EnhancedInputActionIA_ZoomCamera
  (params (ActionValue :type Boolean) (ElapsedSeconds :type Float%20%28double-precision%29) (TriggeredSeconds :type Float%20%28double-precision%29) (InputAction :type Input%20Action%20Object%20Reference :default "/Game/OwnBP/C++/Player_Camera/Inputs/IA_ZoomCamera.IA_ZoomCamera"))
  ;[1 1 1] zoom
  (bind _ascamera_player (Utilities|Casting|CastToCameraPlayer (Pawn|GetControlledPawn)))
  (Class|CameraPlayer|Zoom _ascamera_player))

(event Input|EnhancedActionEvents|EnhancedInputActionIA_UnzoomCamera
  (params (ActionValue :type Boolean) (ElapsedSeconds :type Float%20%28double-precision%29) (TriggeredSeconds :type Float%20%28double-precision%29) (InputAction :type Input%20Action%20Object%20Reference :default "/Game/OwnBP/C++/Player_Camera/Inputs/IA_UnzoomCamera.IA_UnzoomCamera"))
  ;[1 1 1] unzoom
  (bind _ascamera_player (Utilities|Casting|CastToCameraPlayer (Pawn|GetControlledPawn)))
  (Class|CameraPlayer|UnZoom _ascamera_player))

(event Input|EnhancedActionEvents|EnhancedInputActionIA_CancelActionSpawningSystem
  (params (ActionValue :type Boolean) (ElapsedSeconds :type Float%20%28double-precision%29) (TriggeredSeconds :type Float%20%28double-precision%29) (InputAction :type Input%20Action%20Object%20Reference :default "/Game/OwnBP/C++/Player_Camera/Inputs/IA_CancelActionSpawningSystem.IA_CancelActionSpawningSystem"))
  ;[1 1 1] Cancel last action during the spawning system
  (if (Utilities|IsValid (Variables|Default|GetSoldierToSpawn))
    (Class|CameraPlayerController|OnClickCancelLastAction)
    (Actor|GetActorOfClass "/Game/OwnBP/C++/Allies/Preview/BP_TrenchesDefensePreviewCharacter.BP_TrenchesDefensePreviewCharacter_C")
    (Default|CallOnStopSelecting)))

(event EventBeginPlay
  ;[1 1 1] init spawn location
  (bind _returnvalue (Actor|GetActorOfClass "/Game/OwnBP/C++/Field/BP_SoldierDefaultSpawn.BP_SoldierDefaultSpawn_C"))
  (Variables|Default|SetSaveSpawnActorValue (Transformation|GetActorLocation _returnvalue))
  ;[1 1 1] enable enhanced inputs
  (Input|AddMappingContext (PlayerController|LocalPlayerSubsystems|GetEnhancedInputLocalPlayerSubsystem) "/Game/OwnBP/C++/Player_Camera/Inputs/IMC_Player.IMC_Player" 0 "(bIgnoreAllPressedKeysUntilRelease=True,bForceImmediately=False,bNotifyUserSettings=False)")
  ;[1 1 1] widgets
  (bind _returnvalue_2 (UserInterface|CreateWidget "/Game/OwnBP/C++/Allies/Preview/WBP_PreviewCharacterWidget.WBP_PreviewCharacterWidget_C"))
  (UserInterface|Viewport|AddtoViewport _returnvalue_2 0)
  (Widget|SetVisibility _returnvalue_2 "Hidden")
  (bind _returnvalue_3 (UserInterface|CreateWidget "/Game/OwnBP/C++/Allies/General/WBP_GeneralSpeakingWidget.WBP_GeneralSpeakingWidget_C"))
  (UserInterface|Viewport|AddtoViewport _returnvalue_3 0)
  (bind _returnvalue_4 (UserInterface|CreateWidget "/Game/OwnBP/C++/Player_Camera/WBP_BasicInformationWidget.WBP_BasicInformationWidget_C"))
  (UserInterface|Viewport|AddtoViewport _returnvalue_4 0))

(event EventTick
  (params (DeltaSeconds :type Float%20%28single-precision%29)))

(fn ConstructionScript)