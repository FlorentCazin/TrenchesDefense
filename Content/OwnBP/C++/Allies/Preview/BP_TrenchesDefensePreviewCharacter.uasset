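; Preview character for Trenches Defense allies that shows a given soldier's weapon and animation.
; SetPreviewFunction stores the character to preview, spawns its soldier data asset's preview weapon on the RightHandWeapon socket and loops its preview animation.
; StopPreviewFunction clears that reference, stops the animation, then detaches and destroys the weapon.
; The event graph and construction script are empty, so both functions rely on external callers.
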(event EventBeginPlay)

(event Collision|EventActorBeginOverlap
  (params (OtherActor :type Actor%20Object%20Reference)))

(event EventTick
  (params (DeltaSeconds :type Float%20%28single-precision%29)))

(fn ConstructionScript)

(fn SetPreviewFunction
  (params (Character%20to%20preview :type Trenches%20Defense%20Character%20Object%20Reference))
  (Variables|Default|SetCharacterToPreview Character%20to%20preview)
  (bind _returnvalue (Game|SpawnActorfromClass (Variables|/Script/TrenchesDefense.SoldierDataAsset|GetWeaponPreview (Variables|/Script/TrenchesDefense.TrenchesDefenseCharacter|GetSoldierDataAsset (Variables|Default|GetCharacterToPreview))) (Transformation|GetSocketTransform (Variables|Character|GetMesh) "RightHandWeapon" "RTS_World") "Undefined" "MultiplyWithRoot" 0 0))
  (bind _output_get (Variables|Default|SetWeaponAttachedToSocket _returnvalue))
  (Transformation|AttachComponentToComponent _output_get (Variables|Character|GetMesh) "RightHandWeapon" "SnapToTarget" "SnapToTarget" "SnapToTarget" true)
  (Components|Animation|PlayAnimation (Variables|Character|GetMesh) (Variables|/Script/TrenchesDefense.TrenchesDefenseCharacter|GetAnimationPreview (Variables|Default|GetCharacterToPreview)) true))

(fn StopPreviewFunction
  (bind _weaponattachedtosocket (Variables|Default|GetWeaponAttachedToSocket))
  (Variables|Default|SetCharacterToPreview 0)
  (Audio|Components|Audio|Stop (Variables|Character|GetMesh))
  (Transformation|DetachFromActor _weaponattachedtosocket "KeepRelative" "KeepRelative" "KeepRelative")
  (Actor|DestroyActor _weaponattachedtosocket))