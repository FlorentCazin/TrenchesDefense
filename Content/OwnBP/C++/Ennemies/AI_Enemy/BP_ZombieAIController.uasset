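; Zombie AI controller that passes perception updates to its Blackboard for use by the enemy's AI.
; When AIPerception reports a target update, it sets HasLineOfSight to true and stores that actor's location in TargetToReach.
; It does not check whether the stimulus was gained or lost, so this graph never clears the flag.
; BeginPlay, Tick and Possess are empty, and a debug print is left unconnected.
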(event OnTargetPerceptionUpdated(AIPerception)
  (params (Actor :type Actor%20Object%20Reference) (Stimulus :type AI%20Stimulus%20Structure))
  (bind _returnvalue (AI|GetBlackboard 0))
  (AI|Components|Blackboard|SetValueasBool _returnvalue (Variables|Default|GetHasLineOfSight) true)
  (AI|Components|Blackboard|SetValueasVector _returnvalue (Variables|Default|GetTargetToReach) (Transformation|GetActorLocation Actor)))

(event EventBeginPlay)

(event EventTick
  (params (DeltaSeconds :type Float%20%28single-precision%29)))

(event EventPossess
  (params (PossessedPawn :type Pawn%20Object%20Reference)))

(fn ConstructionScript)