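; Camera player controller for placing soldiers with the mouse and handling camera input.
; Left click multi-traces under the cursor after a short delay; if it hits the spawn limitation volume, a soldier spawns at the default spawn and AI-moves to the impact point.
; The mouse wheel zooms the CameraPlayer pawn, and right click only sets a held flag.
; Tick runs a cursor trace with persistent debug drawing, its result unused.
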(event EventBeginPlay)

(event EventTick
  (params (DeltaSeconds :type Float%20%28single-precision%29))
  (bind (_locationx _locationy) (Game|Player|GetMousePosition))
  (bind _returnvalue (Game|GetPlayerController 0))
  (bind _returnvalue_2 (Math|Vector2D|MakeVector2D _locationx _locationy))
  (bind (_worldposition _worlddirection) (Class|GameplayStatics|DeprojectScreentoWorld _returnvalue _returnvalue_2))
  (Collision|LineTraceByChannel (Transformation|GetActorLocation (Game|Player|GetPlayerPawn 0)) (+ _worldposition (* _worlddirection 1e+04)) "TraceTypeQuery1" false 0 "Persistent"))

(event Input|MouseEvents|RightMouseButton
  (params (Key :type Key%20Structure :default "None"))
  ;[1 1 1] rotation giving the priority for the first axe trigged
  (:Pressed
    (Variables|Default|SetRightClickPressed true))
  (:Released
    (Variables|Default|SetRightClickPressed false)))

(event Input|MouseEvents|MouseWheelUp
  (params (Key :type Key%20Structure :default "None"))
  ;[1 1 1] zoom
  (:Pressed
    (bind _ascamera_player (Utilities|Casting|CastToCameraPlayer (Pawn|GetControlledPawn)))
    (Class|CameraPlayer|Zoom _ascamera_player)))

(event Input|MouseEvents|MouseWheelDown
  (params (Key :type Key%20Structure :default "None"))
  ;[1 1 1] unzoom
  (:Pressed
    (bind _ascamera_player (Utilities|Casting|CastToCameraPlayer (Pawn|GetControlledPawn)))
    (Class|CameraPlayer|UnZoom _ascamera_player)))

(event Input|MouseEvents|LeftMouseButton
  (params (Key :type Key%20Structure :default "None"))
  (bind _returnvalue (Game|GetPlayerController 0))
  (bind (_locationx _locationy) (Game|Player|GetMousePosition))
  (bind _returnvalue_2 (Math|Vector2D|MakeVector2D _locationx _locationy))
  (bind (_worldposition _worlddirection) (Class|GameplayStatics|DeprojectScreentoWorld _returnvalue _returnvalue_2))
  ;[1 1 1] Spawn and move the Soldier to is position
  (:Pressed
    ;;[1 1 1] For the BP_limitation boolean
    (Utilities|FlowControl|Delay 0.1)
    ;;[1 1 1] Ignore the characters and the camera limitation
    (bind _returnvalue_3 (Actor|GetActorOfClass "/Game/OwnBP/C++/camera/BP_CameraPlayerLimitation.BP_CameraPlayerLimitation_C"))
    (bind _returnvalue_4 (Actor|GetActorOfClass "/Script/TrenchesDefense.TrenchesDefenseCharacter"))
    (bind _outhits (Collision|MultiLineTraceByChannel (Transformation|GetActorLocation (Game|Player|GetPlayerPawn 0)) (+ _worldposition (* _worlddirection 1e+04)) "TraceTypeQuery1" false (Utilities|Array|MakeArray _returnvalue_4 _returnvalue_3) "None"))
    (for _array_element _outhits
      ;;[1 1 1] Init values in the case we hit the box limitation
      (if (Utilities|ClassIsChildOf (Utilities|GetClass (.HitActor (Collision|BreakHitResult _array_element))) "/Game/OwnBP/C++/Field/BP_LimitationSpawnInProgressToC++NextStape.BP_LimitationSpawnInProgressToC++NextStape_C")
        (Variables|Default|SetSpawningSoldierIsInLimitation true)
        (else
          (Variables|Default|SetSpawningSoldierLocation (.ImpactPoint (Collision|BreakHitResult _array_element))))))
    ;;[1 1 1] If we hit the BoxLimitationSpawn
    (if (Variables|Default|GetSpawningSoldierIsInLimitation)
      (bind _returnvalue_5 (Actor|GetActorOfClass "/Game/OwnBP/C++/Field/BP_SoldierSpawnDefault.BP_SoldierSpawnDefault_C"))
      (bind _returnvalue_6 (Game|SpawnActorfromClass "/Game/OwnBP/C++/Allies/BP_SoldierCharacter.BP_SoldierCharacter_C" (Math|Transform|MakeTransform (Transformation|GetWorldLocation (Variables|/Game/OwnBP/C++/Field/BP_SoldierSpawnDefault.BP_SoldierSpawnDefault_C|GetDefaultSceneRoot _returnvalue_5)) "0, 0, 0" "1.000000,1.000000,1.000000") "Undefined" "MultiplyWithRoot" 0 0))
      (AI|AIMoveTo _returnvalue_6 (Variables|Default|GetSpawningSoldierLocation) 0 5.0 false
        (:then
          (Variables|Default|SetSpawningSoldierIsInLimitation false))))))

(fn ConstructionScript)